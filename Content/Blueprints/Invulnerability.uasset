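; Spinning power-up pickup that grants Quad Damage, Haste or Invulnerability to the player character on overlap.
; The type comes from the name of the static mesh's first material, which selects the index passed to PowerUpOn on MyCharacter_BP.
; The pickup then destroys itself; overlaps from other actors are ignored.
; Tick yaws the actor at RotationSpeed, scaled by delta time.
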(event EventBeginPlay)

(event Collision|EventActorBeginOverlap
  (params (OtherActor :type Actor%20Object%20Reference))
  (bind _asmy_character_bp (Utilities|Casting|CastToMyCharacter_BP OtherActor))
  (switch string (Utilities|GetObjectName (Rendering|Material|GetMaterial (Variables|Default|GetStaticMesh) 0))
    (:Quad_Damage
      (Class|MyCharacter|PowerUpon _asmy_character_bp 1))
    (:Haste
      (Class|MyCharacter|PowerUpon _asmy_character_bp 2))
    (:Invulnerability
      (Class|MyCharacter|PowerUpon _asmy_character_bp 3)))
  (Actor|DestroyActor))

(event EventTick
  (params (DeltaSeconds :type Float%20%28single-precision%29))
  (Class|Actor|AddActorWorldRotation (Math|Rotator|MakeRotator 0.0 0.0 (* DeltaSeconds (Variables|Default|GetRotation%20Speed)))))

(fn ConstructionScript)