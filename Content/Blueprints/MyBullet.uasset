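; MyBullet is a physics-driven projectile actor that damages enemies and destroys targets on impact.
; On spawn it launches itself with a force along its right vector, and quadruples its damage with a Quad Damage sound if the player character's power-up is active.
; On any hit it destroys a Target outright or passes its damage to an Enemy, then destroys itself.
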(event EventBeginPlay
  (Physics|AddForce (Variables|Default|GetBullet) (* (Transformation|GetActorRightVector) 5e+04) "None" false)
  (bind _asmy_character_bp (Utilities|Casting|CastToMyCharacter_BP (Game|Player|GetPlayerPawn 0)))
  (if (== (Variables|/Script/Mutant_Raid.MyCharacter|GetpowerUpActive _asmy_character_bp) 1)
    (Audio|PlaySoundatLocation "/Game/Sound/SFX/Quad_Damage.Quad_Damage" (Transformation|GetActorLocation) "0, 0, 0" 1.0 1.0 0.0 0 0 0)
    (Variables|Default|SetDamage (* (Variables|Default|GetDamage) 4.0))))

(event Collision|EventHit
  (params (MyComp :type Primitive%20Component%20Object%20Reference) (Other :type Actor%20Object%20Reference) (OtherComp :type Primitive%20Component%20Object%20Reference) (bSelfMoved :type Boolean) (HitLocation :type Vector :default "0, 0, 0") (HitNormal :type Vector :default "0, 0, 0") (NormalImpulse :type Vector :default "0, 0, 0") (Hit :type Hit%20Result%20Structure%20%28by%20ref%29))
  (bind _astarget (Utilities|Casting|CastToTarget Other)
    (:then
      (Default|Destroy _astarget))
    (:CastFailed
      (bind _asenemy (Utilities|Casting|CastToEnemy Other)
        (:then
          (Default|GetDamage _asenemy (Variables|Default|GetDamage)))
        (:CastFailed
          _))))
  (Actor|DestroyActor))

(fn ConstructionScript)