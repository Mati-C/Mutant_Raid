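; Base logic for a mutant enemy that chases and attacks the player, either by shooting or by melee.
; Tick checks two radius overlaps to idle, chase by direct location offsets, or attack, driving animation-instance flags.
; Attacks use delay and cooldown, then spawn an aimed bullet or apply damage plus an effect.
; Death decrements the player's mutant count, then destroys the actor, or clears the level (win screen on Level_5) at zero.
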(event Custom|Attack
  (params (Shoot :type Boolean))
  (bind _player (Variables|Default|GetPlayer))
  (bind _ph (Variables|Default|GetPH))
  (bind _returnvalue (Transformation|GetActorLocation _player))
  (bind _returnvalue_2 (Transformation|GetWorldLocation _ph))
  (bind _returnvalue_3 (- _returnvalue _returnvalue_2))
  (bind _returnvalue_4 (Math|Conversions|RotationFromXVector _returnvalue_3))
  (bind (_roll _pitch _yaw) (Math|Rotator|BreakRotator _returnvalue_4))
  (if (not (Variables|Default|GetAttacking))
    (Variables|Default|SetAttacking true)
    (Utilities|FlowControl|Delay (Variables|Default|GetAttack%20Delay))
    (if Shoot
      (Game|SpawnActorfromClass "/Game/Blueprints/EnemyBullet.EnemyBullet_C" (Math|Transform|MakeTransform _returnvalue_2 (Math|Rotator|MakeRotator _roll _pitch (+ _yaw -9e+01))) "Undefined" 0 0)
      (else
        (Class|MyCharacter|Damage (Variables|Default|GetPlayer) (Variables|Default|GetDamage))
        (Class|MyCharacter|PowerUpon (Variables|Default|GetPlayer) (Variables|Default|GetAttack%20Effect))))
    (Utilities|FlowControl|Delay (Variables|Default|GetAttack%20Cooldown))
    (Variables|Default|SetAttacking false)))

(event Custom|Get%20Damage
  (params (Damage :type Float%20%28single-precision%29))
  (bind _output_get (Variables|Default|SetLife (- (Variables|Default|GetLife) Damage)))
  (if (<= _output_get 0.0)
    (CallFunction|SetBools false false true)
    (Utilities|FlowControl|Delay (Variables|Default|GetDeath%20Time))
    (bind _result (Math|Integer|DecrementInt (Variables|/Script/Mutant_Raid.MyCharacter|GetmutantsRemaining (Variables|Default|GetPlayer)))
      (:%20%20
        (if (<= _result 0)
          (bind _returnvalue (Game|GetCurrentLevelName true))
          (if (Utilities|Enum|NotEqual(Enum) _returnvalue "Level_5")
            (Default|LevelClear (Variables|Default|GetPlayer))
            (else
              (Game|OpenLevel(byName) "Win_Game")))
          (else
            (Actor|DestroyActor)))))))

(event Custom|Set%20Bools
  (params (isAttacking :type Boolean) (isMoving :type Boolean) (isDead :type Boolean))
  (bind _anim_instance (Variables|Default|GetAnim%20Instance))
  (Variables|/Script/Mutant_Raid.EnemyAnimInstance|SetisAttacking _anim_instance isAttacking)
  (Variables|/Script/Mutant_Raid.EnemyAnimInstance|SetisMoving _anim_instance isMoving)
  (Variables|/Script/Mutant_Raid.EnemyAnimInstance|SetisDead _anim_instance isDead))

(event EventBeginPlay
  (bind _asmy_character_bp (Utilities|Casting|CastToMyCharacter_BP (Game|Player|GetPlayerPawn 0)))
  (Variables|Default|SetPlayer _asmy_character_bp)
  (bind _asenemy_anim_instance (Utilities|Casting|CastToEnemyAnimInstance (Components|SkeletalMesh|GetAnimInstance (Variables|Default|GetSkeletalMesh))))
  (Variables|Default|SetAnim%20Instance _asenemy_anim_instance)
  (Variables|Default|SetLife (Variables|Default|GetMax%20Life)))

(event EventTick
  (params (DeltaSeconds :type Float%20%28single-precision%29))
  (bind _returnvalue (Transformation|GetActorLocation))
  (bind _player (Variables|Default|GetPlayer))
  (bind _returnvalue_2 (Transformation|GetActorLocation _player))
  (bind _returnvalue_3 (- _returnvalue_2 _returnvalue))
  (bind _returnvalue_4 (Math|Conversions|RotationFromXVector _returnvalue_3))
  (bind (_roll _pitch _yaw) (Math|Rotator|BreakRotator _returnvalue_4))
  (bind _returnvalue_5 (+ _yaw -9e+01))
  (bind _returnvalue_6 (Math|Rotator|MakeRotator _roll 0.0 _returnvalue_5))
  (if (not (Variables|/Script/Mutant_Raid.EnemyAnimInstance|GetisDead (Variables|Default|GetAnim%20Instance)))
    (if (Collision|IsOverlappingActor (Variables|Default|GetAttack%20Radius) (Variables|Default|GetPlayer) :!class /Script/Engine.PrimitiveComponent)
      (CallFunction|SetBools true false false)
      (CallFunction|Attack (Variables|Default|GetShoots))
      (Transformation|SetActorRotation _returnvalue_6)
      (elif (Collision|IsOverlappingActor (Variables|Default|GetChase%20Radius) (Variables|Default|GetPlayer) :!class /Script/Engine.PrimitiveComponent)
        (Transformation|SetActorRotation _returnvalue_6)
        (Transformation|SetActorLocation (+ (Transformation|GetActorLocation) (* (Transformation|GetActorRightVector) (Variables|Default|GetSpeed))) false false)
        (CallFunction|SetBools false true false)
        (else
          (CallFunction|SetBools false false false))))))

(fn ConstructionScript)