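; Spawner is an actor that spawns a random enemy inside a box volume when its Spawn event is called.
; It picks a random class from the Enemies array and a random X and Y within the Volume's scaled extent.
; Z is fixed at the bottom of that extent, relative to the actor's location, and a leftover random Z calculation is unused.
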(event Custom|Spawn
  (bind _volume (Variables|Default|GetVolume))
  (bind _enemies (Variables|Default|GetEnemies))
  (bind _returnvalue (Components|Box|GetScaledBoxExtent _volume))
  (bind (_x _y _z) (Math|Vector|BreakVector _returnvalue))
  (Game|SpawnActorfromClass (Utilities|Array|Get(acopy) _enemies (Math|Random|RandomIntegerinRange 0 (- (Utilities|Array|Length _enemies) 1))) (Math|Conversions|ToTransform(Vector) (+ (Math|Vector|MakeVector (Math|Random|RandomFloatinRange (* -1 _x) _x) (Math|Random|RandomFloatinRange (* -1 _y) _y) (* -1 _z)) (Transformation|GetActorLocation))) "Undefined" 0 0))

(fn ConstructionScript)