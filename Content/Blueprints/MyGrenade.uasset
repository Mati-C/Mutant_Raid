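; A grenade projectile actor that launches itself on spawn and explodes on impact, damaging enemies.
; BeginPlay pushes the Bullet component along the actor's right vector and quadruples damage, with a Quad Damage sound, when the player's power-up is active.
; On hit it spawns a scaled-up explosion, applies damage to every Enemy pawn in a very large sphere overlap, then destroys itself.
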(event EventBeginPlay
  (Physics|AddForce (Variables|Default|GetBullet) (* (Transformation|GetActorRightVector) 2e+06) "None" false)
  (bind _asmy_character_bp (Utilities|Casting|CastToMyCharacter_BP (Game|Player|GetPlayerPawn 0)))
  (if (== (Variables|/Script/Mutant_Raid.MyCharacter|GetpowerUpActive _asmy_character_bp) 1)
    (Audio|PlaySoundatLocation "/Game/Sound/SFX/Quad_Damage.Quad_Damage" (Transformation|GetActorLocation) "0, 0, 0" 1.0 1.0 0.0 0 0 0)
    (Variables|Default|SetDamage (* (Variables|Default|GetDamage) 4.0))))

(event Collision|EventHit
  (params (MyComp :type Primitive%20Component%20Object%20Reference) (Other :type Actor%20Object%20Reference) (OtherComp :type Primitive%20Component%20Object%20Reference) (bSelfMoved :type Boolean) (HitLocation :type Vector :default "0, 0, 0") (HitNormal :type Vector :default "0, 0, 0") (NormalImpulse :type Vector :default "0, 0, 0") (Hit :type Hit%20Result%20Structure%20%28by%20ref%29))
  (Game|SpawnActorfromClass "/Game/Blueprints/Explosion.Explosion_C" (Math|Transform|MakeTransform HitLocation "0, 0, 0" "3.000000,3.000000,3.000000") "Undefined" 0 0)
  (bind _outactors (Collision|SphereOverlapActors (Transformation|GetActorLocation) 2e+05 (Utilities|Array|MakeArray "ObjectTypeQuery3") "/Game/Blueprints/Enemies/Enemy.Enemy_C"))
  (for _array_element _outactors
    (bind _asenemy (Utilities|Casting|CastToEnemy _array_element))
    (Default|GetDamage _asenemy (Variables|Default|GetDamage)))
  (Actor|DestroyActor))

(fn ConstructionScript)